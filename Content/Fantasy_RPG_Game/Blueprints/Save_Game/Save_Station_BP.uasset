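; Save station actor that shows a "press F to save" prompt and enables input while the warrior overlaps its box.
; Pressing F opens the character's attributes widget after a delay; nothing here calls Save_Game.
; Save_Game chains events saving attributes, customization, inventory, location and gate position, then clears the first-play flag.
; Each event separately loads and rewrites the shared slot, or has Save_Game_BP create save data if none exists.
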(event `Save_Game`
  ;[1 1 1] Save_Game_Data
  (`KismetSystemLibrary.Delay` 0.1)
  (`self.Save_Player_Attributes`)
  (`KismetSystemLibrary.Delay` 0.1)
  (`self.Save_Character_Customization`)
  (`KismetSystemLibrary.Delay` 0.1)
  (`self.Save_Player_Inventory`)
  (`KismetSystemLibrary.Delay` 0.1)
  (`self.Save_Player_Location`)
  (`self.Save_Gate_Position`)
  (`self.Set_New_Game_To_False`))

(event `self.Box.OnComponentBeginOverlap`
  (params (OverlappedComponent :type "PrimitiveComponent Object Reference") (OtherActor :type "Actor Object Reference") (OtherComp :type "PrimitiveComponent Object Reference") (OtherBodyIndex :type Integer) (bFromSweep :type Boolean) (SweepResult :type "HitResult Structure (by ref)"))
  ;[1 1 1] Show_Button_Option_When_Collision_Box_Is_Overlapped
  (cast `/Game/Fantasy_RPG_Game/Blueprints/Warrior/Warrior_Character_BP` OtherActor)
  (bind _returnvalue (`|CreateWidget` "/Game/Fantasy_RPG_Game/Widgets/Press_F_To_Save_Game_Widget.Press_F_To_Save_Game_Widget_C" (`GameplayStatics.GetPlayerController` 0)))
  (`UserWidget.AddToViewport` _returnvalue 0)
  (`self.EnableInput` (`GameplayStatics.GetPlayerController` 0)))

(event `self.Box.OnComponentEndOverlap`
  (params (OverlappedComponent :type "PrimitiveComponent Object Reference") (OtherActor :type "Actor Object Reference") (OtherComp :type "PrimitiveComponent Object Reference") (OtherBodyIndex :type Integer))
  ;[1 1 1] Remove_Button_Option_When_Overlapping_Ends
  (cast `/Game/Fantasy_RPG_Game/Blueprints/Warrior/Warrior_Character_BP` OtherActor)
  (`Widget.RemoveFromParent` (stale `self.Box.OnComponentBeginOverlap` _returnvalue))
  (`self.DisableInput` (`GameplayStatics.GetPlayerController` 0)))

(event `Key|F`
  (params (Key :type "Key Structure"))
  ;[1 1 1] Show_Attribute_Menu
  (:`Pressed`
    (`KismetSystemLibrary.Delay` 1.0)
    (bind _aswarrior_character_bp (cast `/Game/Fantasy_RPG_Game/Blueprints/Warrior/Warrior_Character_BP` (`GameplayStatics.GetPlayerCharacter` 0)))
    (`/Game/Fantasy_RPG_Game/Blueprints/Warrior/Warrior_Character_BP.Create_Attributes_Widget` _aswarrior_character_bp)))

(event `Save_Player_Attributes`
  ;[1 1 1] Save_Player_Attributes
  (bind _returnvalue (`GameplayStatics.DoesSaveGameExist` "Save_Game"))
  (if _returnvalue
    (bind _returnvalue_2 (`GameplayStatics.LoadGameFromSlot` "Save_Game"))
    (bind _assave_game_data (cast `/Game/Fantasy_RPG_Game/Save_Games/Save_Game_Data` _returnvalue_2))
    (bind _aswarrior_character_bp (cast `/Game/Fantasy_RPG_Game/Blueprints/Warrior/Warrior_Character_BP` (`GameplayStatics.GetPlayerCharacter` 0)))
    (set `/Game/Fantasy_RPG_Game/Save_Games/Save_Game_Data.Light_Attack_Stamina` (`/Game/Fantasy_RPG_Game/Blueprints/Warrior/Warrior_Character_BP.Light_Attack_Stamina` _aswarrior_character_bp) _assave_game_data)
    (set `/Game/Fantasy_RPG_Game/Save_Games/Save_Game_Data.Stamina_Regenaration_Rate` (`/Game/Fantasy_RPG_Game/Blueprints/Warrior/Warrior_Character_BP.Stamina_Regeneration_Rate` _aswarrior_character_bp) _assave_game_data)
    (set `/Game/Fantasy_RPG_Game/Save_Games/Save_Game_Data.XP_Points` (`/Game/Fantasy_RPG_Game/Blueprints/Warrior/Warrior_Character_BP.XP_POINTS` _aswarrior_character_bp) _assave_game_data)
    (set `/Game/Fantasy_RPG_Game/Save_Games/Save_Game_Data.Damage_Amount_From_Zombie` (`/Game/Fantasy_RPG_Game/Blueprints/Warrior/Warrior_Character_BP.Damage_Amount_From_Zombie` _aswarrior_character_bp) _assave_game_data)
    (set `/Game/Fantasy_RPG_Game/Save_Games/Save_Game_Data.Damage_Amount_From_Dragon` (`/Game/Fantasy_RPG_Game/Blueprints/Warrior/Warrior_Character_BP.Damage_Amount_From_Dragon_Bite` _aswarrior_character_bp) _assave_game_data)
    (set `/Game/Fantasy_RPG_Game/Save_Games/Save_Game_Data.Health_Bar_Size` (`/Game/Fantasy_RPG_Game/Blueprints/Warrior/Warrior_Character_BP.Health_Bar_Size` _aswarrior_character_bp) _assave_game_data)
    (set `/Game/Fantasy_RPG_Game/Save_Games/Save_Game_Data.Stamina_Bar_Size` (`/Game/Fantasy_RPG_Game/Blueprints/Warrior/Warrior_Character_BP.Stamina_Bar_Size` _aswarrior_character_bp) _assave_game_data)
    (set `/Game/Fantasy_RPG_Game/Save_Games/Save_Game_Data.Player_Level` (`/Game/Fantasy_RPG_Game/Blueprints/Warrior/Warrior_Character_BP.Player_Level` _aswarrior_character_bp) _assave_game_data)
    (`GameplayStatics.SaveGameToSlot` _returnvalue_2 "Save_Game")
    (`KismetSystemLibrary.Delay` 0.2)
    (else
      (bind _outactors (`GameplayStatics.GetAllActorsOfClass` "/Game/Fantasy_RPG_Game/Blueprints/Save_Game/Save_Game_BP.Save_Game_BP_C"))
      (`/Game/Fantasy_RPG_Game/Blueprints/Save_Game/Save_Game_BP.Create_Save_Data` (`|GetArrayItem` _outactors)))))

(event `Save_Character_Customization`
  ;[1 1 1] Save_Character_Customization
  (bind _returnvalue (`GameplayStatics.DoesSaveGameExist` "Save_Game"))
  (if _returnvalue
    (bind _returnvalue_2 (`GameplayStatics.LoadGameFromSlot` "Save_Game"))
    (bind _assave_game_data (cast `/Game/Fantasy_RPG_Game/Save_Games/Save_Game_Data` _returnvalue_2))
    (bind _aswarrior_character_bp (cast `/Game/Fantasy_RPG_Game/Blueprints/Warrior/Warrior_Character_BP` (`GameplayStatics.GetPlayerCharacter` 0)))
    (set `/Game/Fantasy_RPG_Game/Save_Games/Save_Game_Data.Body_Fat` (`/Game/Fantasy_RPG_Game/Blueprints/Warrior/Warrior_Character_BP.Body_Fat` _aswarrior_character_bp) _assave_game_data)
    (set `/Game/Fantasy_RPG_Game/Save_Games/Save_Game_Data.Face_Shape` (`/Game/Fantasy_RPG_Game/Blueprints/Warrior/Warrior_Character_BP.Face_Shape` _aswarrior_character_bp) _assave_game_data)
    (set `/Game/Fantasy_RPG_Game/Save_Games/Save_Game_Data.Face_Roundness` (`/Game/Fantasy_RPG_Game/Blueprints/Warrior/Warrior_Character_BP.Face_Roundness` _aswarrior_character_bp) _assave_game_data)
    (set `/Game/Fantasy_RPG_Game/Save_Games/Save_Game_Data.Cheek_Size` (`/Game/Fantasy_RPG_Game/Blueprints/Warrior/Warrior_Character_BP.Cheek_Size` _aswarrior_character_bp) _assave_game_data)
    (set `/Game/Fantasy_RPG_Game/Save_Games/Save_Game_Data.Nose_Size` (`/Game/Fantasy_RPG_Game/Blueprints/Warrior/Warrior_Character_BP.Nose_Size` _aswarrior_character_bp) _assave_game_data)
    (set `/Game/Fantasy_RPG_Game/Save_Games/Save_Game_Data.Jaw_Size` (`/Game/Fantasy_RPG_Game/Blueprints/Warrior/Warrior_Character_BP.Jaw_Size` _aswarrior_character_bp) _assave_game_data)
    (set `/Game/Fantasy_RPG_Game/Save_Games/Save_Game_Data.Lip_Size` (`/Game/Fantasy_RPG_Game/Blueprints/Warrior/Warrior_Character_BP.Lip_Size` _aswarrior_character_bp) _assave_game_data)
    (set `/Game/Fantasy_RPG_Game/Save_Games/Save_Game_Data.Eye_Shape` (`/Game/Fantasy_RPG_Game/Blueprints/Warrior/Warrior_Character_BP.Eye_Shape` _aswarrior_character_bp) _assave_game_data)
    (set `/Game/Fantasy_RPG_Game/Save_Games/Save_Game_Data.Skin_Color` (`/Game/Fantasy_RPG_Game/Blueprints/Warrior/Warrior_Character_BP.Skin_Color` _aswarrior_character_bp) _assave_game_data)
    (`GameplayStatics.SaveGameToSlot` _returnvalue_2 "Save_Game")
    (else
      (bind _outactors (`GameplayStatics.GetAllActorsOfClass` "/Game/Fantasy_RPG_Game/Blueprints/Save_Game/Save_Game_BP.Save_Game_BP_C"))
      (`/Game/Fantasy_RPG_Game/Blueprints/Save_Game/Save_Game_BP.Create_Save_Data` (`|GetArrayItem` _outactors)))))

(event `Save_Player_Inventory`
  ;[1 1 1] Save_Inventory
  (bind _returnvalue (`GameplayStatics.DoesSaveGameExist` "Save_Game"))
  (if _returnvalue
    (bind _returnvalue_2 (`GameplayStatics.LoadGameFromSlot` "Save_Game"))
    (bind _assave_game_data (cast `/Game/Fantasy_RPG_Game/Save_Games/Save_Game_Data` _returnvalue_2))
    (bind _aswarrior_character_bp (cast `/Game/Fantasy_RPG_Game/Blueprints/Warrior/Warrior_Character_BP` (`GameplayStatics.GetPlayerCharacter` 0)))
    (set `/Game/Fantasy_RPG_Game/Save_Games/Save_Game_Data.Ancient_Chest_Armor_Selected` (`/Game/Fantasy_RPG_Game/Blueprints/Warrior/Warrior_Character_BP.Ancient_Chest_Armor_Selected` _aswarrior_character_bp) _assave_game_data)
    (set `/Game/Fantasy_RPG_Game/Save_Games/Save_Game_Data.Leather_Chest_Armor_Selected` (`/Game/Fantasy_RPG_Game/Blueprints/Warrior/Warrior_Character_BP.Leather _Chest_Armor_Selected` _aswarrior_character_bp) _assave_game_data)
    (set `/Game/Fantasy_RPG_Game/Save_Games/Save_Game_Data.Ancient_Bottoms_Selected` (`/Game/Fantasy_RPG_Game/Blueprints/Warrior/Warrior_Character_BP.Ancient_Bottoms_Selected` _aswarrior_character_bp) _assave_game_data)
    (set `/Game/Fantasy_RPG_Game/Save_Games/Save_Game_Data.Leather_Bottoms_Selected` (`/Game/Fantasy_RPG_Game/Blueprints/Warrior/Warrior_Character_BP.Leather _Bottoms_Selected` _aswarrior_character_bp) _assave_game_data)
    (set `/Game/Fantasy_RPG_Game/Save_Games/Save_Game_Data.Short_Hair_Selected` (`/Game/Fantasy_RPG_Game/Blueprints/Warrior/Warrior_Character_BP.Short_Hair_Selected` _aswarrior_character_bp) _assave_game_data)
    (set `/Game/Fantasy_RPG_Game/Save_Games/Save_Game_Data.Long_Hair_Selected` (`/Game/Fantasy_RPG_Game/Blueprints/Warrior/Warrior_Character_BP.Long_Hair_Selected` _aswarrior_character_bp) _assave_game_data)
    (set `/Game/Fantasy_RPG_Game/Save_Games/Save_Game_Data.Gauntlets_Selected` (`/Game/Fantasy_RPG_Game/Blueprints/Warrior/Warrior_Character_BP.Gauntlets_Selected` _aswarrior_character_bp) _assave_game_data)
    (set `/Game/Fantasy_RPG_Game/Save_Games/Save_Game_Data.Chese_Underwear_Selected` (`/Game/Fantasy_RPG_Game/Blueprints/Warrior/Warrior_Character_BP.Chest_Underwear_Selected` _aswarrior_character_bp) _assave_game_data)
    (set `/Game/Fantasy_RPG_Game/Save_Games/Save_Game_Data.Bottom_Underwear_Selected` (`/Game/Fantasy_RPG_Game/Blueprints/Warrior/Warrior_Character_BP.Bottom_Underwear_Selected` _aswarrior_character_bp) _assave_game_data)
    (set `/Game/Fantasy_RPG_Game/Save_Games/Save_Game_Data.No_Gauntlets_Selected` (`/Game/Fantasy_RPG_Game/Blueprints/Warrior/Warrior_Character_BP.No_Gauntlets_Selected` _aswarrior_character_bp) _assave_game_data)
    (set `/Game/Fantasy_RPG_Game/Save_Games/Save_Game_Data.Elemental_Sword_Selected` (`/Game/Fantasy_RPG_Game/Blueprints/Warrior/Warrior_Character_BP.Elemental_Sword_Selected` _aswarrior_character_bp) _assave_game_data)
    (set `/Game/Fantasy_RPG_Game/Save_Games/Save_Game_Data.Iron_Sword_Selected` (`/Game/Fantasy_RPG_Game/Blueprints/Warrior/Warrior_Character_BP.Iron_Sword_Selected` _aswarrior_character_bp) _assave_game_data)
    (set `/Game/Fantasy_RPG_Game/Save_Games/Save_Game_Data.Iron_Shield_Selected` (`/Game/Fantasy_RPG_Game/Blueprints/Warrior/Warrior_Character_BP.Iron_Shield_Selected` _aswarrior_character_bp) _assave_game_data)
    (set `/Game/Fantasy_RPG_Game/Save_Games/Save_Game_Data.Elemental_Shield_Selected` (`/Game/Fantasy_RPG_Game/Blueprints/Warrior/Warrior_Character_BP.Elemental_Shield_Selected` _aswarrior_character_bp) _assave_game_data)
    (set `/Game/Fantasy_RPG_Game/Save_Games/Save_Game_Data.Bomb_Selected` (`/Game/Fantasy_RPG_Game/Blueprints/Warrior/Warrior_Character_BP.Bomb_Selected` _aswarrior_character_bp) _assave_game_data)
    (set `/Game/Fantasy_RPG_Game/Save_Games/Save_Game_Data.Health_Potion_Selected` (`/Game/Fantasy_RPG_Game/Blueprints/Warrior/Warrior_Character_BP.Health_Potion_Selected` _aswarrior_character_bp) _assave_game_data)
    (set `/Game/Fantasy_RPG_Game/Save_Games/Save_Game_Data.Weapon_1_Current_Index` (`/Game/Fantasy_RPG_Game/Blueprints/Warrior/Warrior_Character_BP.Weapon_Current_Index` _aswarrior_character_bp) _assave_game_data)
    (set `/Game/Fantasy_RPG_Game/Save_Games/Save_Game_Data.Weapon_2_Current_Index` (`/Game/Fantasy_RPG_Game/Blueprints/Warrior/Warrior_Character_BP.Weapon_2_Current_Index` _aswarrior_character_bp) _assave_game_data)
    (`GameplayStatics.SaveGameToSlot` _returnvalue_2 "Save_Game")
    (else
      (bind _outactors (`GameplayStatics.GetAllActorsOfClass` "/Game/Fantasy_RPG_Game/Blueprints/Save_Game/Save_Game_BP.Save_Game_BP_C"))
      (`/Game/Fantasy_RPG_Game/Blueprints/Save_Game/Save_Game_BP.Create_Save_Data` (`|GetArrayItem` _outactors)))))

(event `Save_Player_Location`
  ;[1 1 1] Save_Player_Location
  (bind _returnvalue (`GameplayStatics.DoesSaveGameExist` "Save_Game"))
  (if _returnvalue
    (bind _returnvalue_2 (`GameplayStatics.LoadGameFromSlot` "Save_Game"))
    (bind _assave_game_data (cast `/Game/Fantasy_RPG_Game/Save_Games/Save_Game_Data` _returnvalue_2))
    (bind _aswarrior_character_bp (cast `/Game/Fantasy_RPG_Game/Blueprints/Warrior/Warrior_Character_BP` (`GameplayStatics.GetPlayerCharacter` 0)))
    (set `/Game/Fantasy_RPG_Game/Save_Games/Save_Game_Data.Save_Player_Location` (`SceneComponent.K2_GetComponentToWorld` (`Character.CapsuleComponent` _aswarrior_character_bp)) _assave_game_data)
    (`GameplayStatics.SaveGameToSlot` _assave_game_data "Save_Game")
    (`KismetSystemLibrary.Delay` 0.2)
    (else
      (bind _outactors (`GameplayStatics.GetAllActorsOfClass` "/Game/Fantasy_RPG_Game/Blueprints/Save_Game/Save_Game_BP.Save_Game_BP_C"))
      (`/Game/Fantasy_RPG_Game/Blueprints/Save_Game/Save_Game_BP.Create_Save_Data` (`|GetArrayItem` _outactors)))))

(event `Set_New_Game_To_False`
  ;[1 1 1] Set_New_Game_To_False
  (bind _returnvalue (`GameplayStatics.DoesSaveGameExist` "Save_Game"))
  (if _returnvalue
    (bind _returnvalue_2 (`GameplayStatics.LoadGameFromSlot` "Save_Game"))
    (bind _assave_game_data (cast `/Game/Fantasy_RPG_Game/Save_Games/Save_Game_Data` _returnvalue_2))
    (set `/Game/Fantasy_RPG_Game/Save_Games/Save_Game_Data.First_Play?` false _assave_game_data)
    (`GameplayStatics.SaveGameToSlot` _assave_game_data "Save_Game")
    (else
      (bind _outactors (`GameplayStatics.GetAllActorsOfClass` "/Game/Fantasy_RPG_Game/Blueprints/Save_Game/Save_Game_BP.Save_Game_BP_C"))
      (`/Game/Fantasy_RPG_Game/Blueprints/Save_Game/Save_Game_BP.Create_Save_Data` (`|GetArrayItem` _outactors)))))

(event `Save_Gate_Position`
  ;[1 1 1] Save_Gate_Position(Gate is in the starter map)
  (bind _returnvalue (`GameplayStatics.DoesSaveGameExist` "Save_Game"))
  (if _returnvalue
    (bind _returnvalue_2 (`GameplayStatics.LoadGameFromSlot` "Save_Game"))
    (bind _assave_game_data (cast `/Game/Fantasy_RPG_Game/Save_Games/Save_Game_Data` _returnvalue_2))
    (set `/Game/Fantasy_RPG_Game/Save_Games/Save_Game_Data.Gate_Position` (`self.Gate_Position`) _assave_game_data)
    (`GameplayStatics.SaveGameToSlot` _assave_game_data "Save_Game")
    (else
      (bind _outactors (`GameplayStatics.GetAllActorsOfClass` "/Game/Fantasy_RPG_Game/Blueprints/Save_Game/Save_Game_BP.Save_Game_BP_C"))
      (`/Game/Fantasy_RPG_Game/Blueprints/Save_Game/Save_Game_BP.Create_Save_Data` (`|GetArrayItem` _outactors)))))

(fn `UserConstructionScript`)
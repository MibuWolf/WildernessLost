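; Zombie enemy character that wanders the navmesh until it sees or is hit by the player, then chases and attacks.
; PawnSensing starts a self-calling Delay loop that drives facing and AIMoveTo; reaching the player opens a timed weapon overlap window, then randomly retries or backs off.
; Sword hits drain a floating health bar behind timed debounce flags.
; Death randomly kneels or kills outright, ending in ragdoll, player XP and destruction.
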(event `Face_Player`
  (bind (_returnvalue_x _returnvalue_y _returnvalue_z) (`KismetMathLibrary.BreakVector` (`self.K2_GetActorLocation` (`GameplayStatics.GetPlayerCharacter` 0))))
  ;[1 1 1] Face_Player
  (if (`self.Can Face Player`)
    (`self.K2_SetActorRotation` (`KismetMathLibrary.FindLookAtRotation` (`self.K2_GetActorLocation`) (`KismetMathLibrary.MakeVector` 0.0 0.0 _returnvalue_z)))))

(event `self.PawnSensing.OnSeePawn`
  (params (Pawn :type "Pawn Object Reference"))
  ;[1 1 1] Pawn_Sensing_(If Player is seen)
  (cast `/Game/Fantasy_RPG_Game/Blueprints/Warrior/Warrior_Character_BP` Pawn)
  (`self.Initialize`)
  (`KismetSystemLibrary.Delay` 0.2)
  (set `self.Follow_Player` true))

(event `Successfully_Moved_to_Player`
  ;[1 1 1] Initiate_Attack
  (if (`self.Attack1`)
    _
    (elif (not (`self.Withdraw_Attack`))
      (set `self.Attack1` true)
      (`|ExecutionSequence`
        (:`then_1`
          ;[1 1 1] Randomly_Select_Next_Action
          (`KismetSystemLibrary.Delay` 1.0)
          (switch `int` (`KismetMathLibrary.RandomInteger` 2)
            (:`Default`
              ;[1 1 1] Call_Reinitialize
              (set `self.Attack1` false)
              (`self.ReInitialize`))
            (:`0`
              ;[1 1 1] Withdraw_Attack_&_Reinitialize
              (set `self.Withdraw_Attack` true)
              (set `self.Attack1` false)
              (`KismetSystemLibrary.Delay` 4.0)
              (set `self.Withdraw_Attack` false)
              (`self.ReInitialize`))))
        (:`then_2`
          ;[1 1 1] Open_and_Close_Attack_Collision_Window
          (`KismetSystemLibrary.Delay` 0.5)
          (set `self.Attack_Collision_Window` true)
          (`KismetSystemLibrary.Delay` 0.4)
          (set `self.Attack_Collision_Window` false))))))

(event `self.ReceiveBeginPlay`
  ;[1 1 1] Attach_Weapon
  (`SceneComponent.K2_AttachToComponent` (`self.WeaponSkeletalMesh`) (`self.Mesh`) "Weapon1" "SnapToTarget" "SnapToTarget" "SnapToTarget" true))

(event `Move_To_Player`
  ;[1 1 1] Move_To_Player
  (set `self.Root_Motion_Walk` true)
  (`|AIMoveTo` self (`SceneComponent.K2_GetComponentLocation` (`Character.Mesh` (`GameplayStatics.GetPlayerCharacter` 0))) null (`self.Acceptance radius`)
    (:`OnSuccess`
      (`self.Successfully_Moved_to_Player`))))

(event `ReInitialize`
  ;[1 1 1] Follow_The_Player_Or_Wonder_Aimlessly
  (if (`self.Follow_Player`) :!label _label
    (`self.Face_Player`)
    (`self.Move_To_Player`)
    (else
      (`self.Wonder_Aimlessly`))))

(event `self.Weapon_Collision_Box.OnComponentBeginOverlap`
  (params (OverlappedComponent :type "PrimitiveComponent Object Reference") (OtherActor :type "Actor Object Reference") (OtherComp :type "PrimitiveComponent Object Reference") (OtherBodyIndex :type Integer) (bFromSweep :type Boolean) (SweepResult :type "HitResult Structure (by ref)"))
  ;[1 1 1] Check_If_Weapon_Has_Collided_With_Player
  (if (`self.Attack1`)
    ;[1 1 1] Cast the hit to the Player
    (bind _aswarrior_character_bp (cast `/Game/Fantasy_RPG_Game/Blueprints/Warrior/Warrior_Character_BP` OtherActor))
    (if (`self.Attack_Collision_Window`)
      (`/Engine/EditorBlueprintResources/StandardMacros.DoOnce` false :!label _label_2
        (:`Completed`
          (if (`self.Hit`)
            _
            (elif (not (`self.Is_Dying`))
              (`/Game/Fantasy_RPG_Game/Blueprints/Warrior/Warrior_Character_BP.Hit_By_Zombie1` _aswarrior_character_bp)
              (`KismetSystemLibrary.Delay` 0.4)
              (`self.Reset_Do_Once`))))))))

(event `Initialize`
  ;[1 1 1] Initialize
  (if (not (`self.Is_Dying`))
    (`|ExecutionSequence`
      (:`then_0`
        (goto _label))
      (:`then_1`
        ;[1 1 1] Follow_The_Player_Or_Wonder_Aimlessly
        (if (`self.Can Face Player`)
          (`self.Face_Player`)))
      (:`then_2`
        ;[1 1 1] Full_Reinitialization_Every_O.2_Seconds_to_Update_The_BP
        (`KismetSystemLibrary.Delay` 0.02)
        (`self.Initialize`)))))

(event `Reset_Do_Once`
  ;[1 1 1] Cast the hit to the Player
  (goto _label_2 :!via `Reset`))

(event `Wonder_Aimlessly`
  ;[1 1 1] Wonder_Aimlessly
  (if (`self.Can Move`)
    (set `self.Can Move` false)
    (`|AIMoveTo` self (`NavigationSystem.K2_GetRandomLocationInNavigableRadius` (`SceneComponent.K2_GetComponentLocation` (`self.CapsuleComponent`)) 3000.0) null 220.0
      (:`OnSuccess`
        _)
      (:`OnFail`
        _))
    (set `self.Can Move` true)))

(event `Disable_Player_Hit`
  ;[1 1 1] Disable_Player_Hit
  (`KismetSystemLibrary.Delay` 0.01)
  (set `self.Disable Hit by  Sword` true)
  (`KismetSystemLibrary.Delay` 0.65)
  (set `self.Disable Hit by  Sword` false)
  (set `self.Hit` false))

(event `Disable_Health_Reduction`
  ;[1 1 1] Temporalily_Disable_Health_Reduction (To Avoid multiple hit detections from a single attack)
  (set `self.Can_Reduce_Health` false)
  (`KismetSystemLibrary.Delay` 0.5)
  (set `self.Can_Reduce_Health` true))

(event `Hit By Sword`
  ;[1 1 1] Hit_By_Player
  (`|ExecutionSequence`
    (:`then_0`
      (`self.Play_Hit_Sounds`)
      (if (`self.Can_Reduce_Health`)
        (`|ExecutionSequence`
          (:`then_0`
            (`self.Disable_Health_Reduction`))
          (:`then_1`
            (`self.Reduce_Health`))
          (:`then_2`
            (`self.Show_Health_Bar`)))))
    (:`then_1`
      (if (not (`self.Follow_Player`))
        (set `self.Follow_Player` true)))))

(event `Death`
  ;[1 1 1] Call_Death_Events
  (if (`self.Can_Execute`)
    (`self.Kill`)
    (else
      (switch `int` (`KismetMathLibrary.RandomInteger` 2)
        (:`Default`
          (`self.Kneel`))
        (:`0`
          (`self.Kill`))))))

(event `Check_Player_Attack`
  ;[1 1 1] Check_Player_Attack
  (bind _aswarrior_character_bp (cast `/Game/Fantasy_RPG_Game/Blueprints/Warrior/Warrior_Character_BP` (`GameplayStatics.GetPlayerCharacter` 0)))
  (`|ExecutionSequence`
    (:`then_1`
      (set `self.Hit` true)
      (if (`/Game/Fantasy_RPG_Game/Blueprints/Warrior/Warrior_Character_BP.Light_attack_2` _aswarrior_character_bp)
        (set `self.Hit` false)
        (`KismetSystemLibrary.Delay` 0.01)
        (set `self.Disable Hit by  Sword` true)
        (`KismetSystemLibrary.Delay` 0.65)
        (set `self.Disable Hit by  Sword` false)))))

(event `Reduce_Health`
  ;[1 1 1] Reduce_Health
  (if (`self.Is_Dead`)
    _
    (elif (not (`self.Disable Hit by  Sword`))
      (set `self.Zombie_Health` (- (`self.Zombie_Health`) 0.45))
      (`/Engine/EditorBlueprintResources/StandardMacros.CompareFloat` (`self.Zombie_Health`) 0.01
        (:`>`
          (`|ExecutionSequence`
            (:`then_0`
              (`self.Disable_Player_Hit`))
            (:`then_1`
              (`self.Check_Player_Attack`))
            (:`then_2`
              (`self.Update_Health_Bar`))))
        (:`<`
          ;[1 1 1] Initiate_Zombie_Death
          (`self.Death`))))))

(event `Kneel`
  ;[1 1 1] Kneel_Before_Death_&_Disable_Movement
  (`|ExecutionSequence`
    (:`then_0`
      (`KismetSystemLibrary.Delay` 0.1)
      (set `self.Can_Execute` true))
    (:`then_1`
      (set `self.Is_Dying` true)
      (`KismetSystemLibrary.Delay` 1.3)
      (if true
        (`CharacterMovementComponent.DisableMovement` (`self.CharacterMovement`))
        (`KismetSystemLibrary.Delay` 6.0)
        (`self.Activate_Rag_Doll`)))))

(event `Update_Health_Bar`
  ;[1 1 1] Update_Health_Bar
  (bind _aszombie_health_widget (cast `/Game/Fantasy_RPG_Game/Widgets/Zombie_Health_Widget` (`WidgetComponent.GetUserWidgetObject` (`self.HealthBar`))))
  (set `/Game/Fantasy_RPG_Game/Widgets/Zombie_Health_Widget.Health` (`self.Zombie_Health`) _aszombie_health_widget))

(event `Show_Health_Bar`
  ;[1 1 1] Show_Floating_Health_Bar
  (`SceneComponent.SetVisibility` (`self.HealthBar`) true false))

(event `Kill`
  ;[1 1 1] Kill_Zombie_&_Hide_Health_Widget
  (`Widget.SetVisibility` (`/Game/Fantasy_RPG_Game/Widgets/Zombie_Health_Widget.Health_Bar` (stale `Update_Health_Bar` _aszombie_health_widget)) "Hidden")
  (set `self.Is_Dead` true)
  ;[1 1 1] Activate_Rag_Doll
  (`KismetSystemLibrary.Delay` 0.6)
  (`PrimitiveComponent.SetSimulatePhysics` (`self.Mesh`) true :!label _label_3)
  (`|ExecutionSequence`
    (:`then_0`
      ;[1 1 1] Give_Player_120_Points
      (bind _aswarrior_character_bp (cast `/Game/Fantasy_RPG_Game/Blueprints/Warrior/Warrior_Character_BP` (`GameplayStatics.GetPlayerCharacter` 0)))
      (`/Engine/EditorBlueprintResources/StandardMacros.DoOnce` false
        (:`Completed`
          (set `/Game/Fantasy_RPG_Game/Blueprints/Warrior/Warrior_Character_BP.XP_POINTS` (+ (`/Game/Fantasy_RPG_Game/Blueprints/Warrior/Warrior_Character_BP.XP_POINTS` _aswarrior_character_bp) 120.0) _aswarrior_character_bp))))
    (:`then_1`
      ;[1 1 1] Destroy_Zombie_BP_Actor
      (`PrimitiveComponent.SetCollisionEnabled` (`self.CapsuleComponent`) "NoCollision")
      (`KismetSystemLibrary.Delay` 5.0)
      (`self.K2_DestroyActor`))))

(event `Play_Hit_Sounds`
  ;[1 1 1] Hit_Sounds
  (switch `int` (`KismetMathLibrary.RandomInteger` 2)
    (:`Default`
      (`GameplayStatics.PlaySound2D` "/Game/Fantasy_RPG_Game/Sound/Effects/stab3_A.stab3_A"))
    (:`0`
      (`GameplayStatics.PlaySound2D` "/Game/Fantasy_RPG_Game/Sound/Effects/Stab1_A.Stab1_A")))
  (`GameplayStatics.PlaySound2D` "/Game/Fantasy_RPG_Game/Sound/Zombie/Zombie_Hit_A.Zombie_Hit_A"))

(event `Activate_Rag_Doll`
  ;[1 1 1] Activate_Rag_Doll
  (goto _label_3))

(fn `UserConstructionScript`)
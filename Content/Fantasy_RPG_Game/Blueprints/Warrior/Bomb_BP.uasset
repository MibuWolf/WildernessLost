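; Warrior's bomb projectile that explodes on its first bounce, damaging zombies, Blood Dragons and destructible actors.
; On first tick it sets launch velocity, with vertical speed scaled from the player's clamped Elevation.
; The bounce briefly inflates the ExplosionRadius sphere so overlap events deliver hits, alongside particles, sound, radial impulse and camera shake.
; A Hit event removes the radius and force components after short delays, then destroys the actor.
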(event `self.ReceiveTick`
  (params (DeltaSeconds :type "Float (single-precision)"))
  ;[1 1 1] Check_Player_Camera_Elevation
  (bind _aswarrior_character_bp (cast `/Game/Fantasy_RPG_Game/Blueprints/Warrior/Warrior_Character_BP` (`GameplayStatics.GetPlayerCharacter` 0)))
  (`/Engine/EditorBlueprintResources/StandardMacros.DoOnce` false
    (:`Completed`
      (`ProjectileMovementComponent.SetVelocityInLocalSpace` (`self.ProjectileMovement`) (`KismetMathLibrary.MakeVector` 1000.0 0.0 (* (`KismetMathLibrary.FClamp` (`/Game/Fantasy_RPG_Game/Blueprints/Warrior/Warrior_Character_BP.Elevation` _aswarrior_character_bp) 1.0 10.0) 80.0))))))

(event `self.ProjectileMovement.OnProjectileBounce`
  (params (ImpactResult :type "HitResult Structure (by ref)") (ImpactVelocity :type "Vector Structure (by ref)"))
  (bind _explosion_radius (`self.Explosion_Radius`))
  ;[1 1 1] Explode_On_Bounce
  (`/Engine/EditorBlueprintResources/StandardMacros.DoOnce` false
    (:`Completed`
      (bind _returnvalue (`GameplayStatics.SpawnEmitterAtLocation` "/Game/Fantasy_RPG_Game/Effects/Sparks_Particles.Sparks_Particles" (`SceneComponent.K2_GetComponentLocation` (`self.Bomb`)) (struct) (20.0 20.0 20.0)))
      (`SphereComponent.SetSphereRadius` _explosion_radius 480.0 true)
      (`GameplayStatics.PlaySound2D` "/Game/Fantasy_RPG_Game/Sound/Effects/Explosion_A.Explosion_A")
      (`KismetSystemLibrary.Delay` 0.02)
      (`RadialForceComponent.FireImpulse` (`self.RadialForce`))
      (`GameplayStatics.PlayWorldCameraShake` "/Game/Fantasy_RPG_Game/Blueprints/Warrior/Camera_Shake_Attack_BP.Camera_Shake_Attack_BP_C" (`SceneComponent.K2_GetComponentLocation` (`Character.Mesh` (`GameplayStatics.GetPlayerCharacter` 0))) 0.0 5000.0 1.0 true)
      (`SphereComponent.SetSphereRadius` _explosion_radius 5.0 true)
      (`KismetSystemLibrary.Delay` 0.5)
      (`ActorComponent.Deactivate` _returnvalue))))

(event `self.Explosion_Radius.OnComponentBeginOverlap`
  (params (OverlappedComponent :type "PrimitiveComponent Object Reference") (OtherActor :type "Actor Object Reference") (OtherComp :type "PrimitiveComponent Object Reference") (OtherBodyIndex :type Integer) (bFromSweep :type Boolean) (SweepResult :type "HitResult Structure (by ref)"))
  ;[1 1 1] Destroy/Damage_Actors_In_Radius
  (`|ExecutionSequence`
    (:`then_0`
      (bind _aszombie_bp (cast `/Game/Fantasy_RPG_Game/Blueprints/Zombie/Zombie_BP` OtherActor))
      (`/Game/Fantasy_RPG_Game/Blueprints/Zombie/Zombie_BP.Power_1_Hit` _aszombie_bp)
      (`KismetSystemLibrary.Delay` 0.01)
      (`RadialForceComponent.FireImpulse` (`self.RadialForce`))
      (`GameplayStatics.PlaySoundAtLocation` "/Game/Fantasy_RPG_Game/Sound/Effects/Explosion_A.Explosion_A" (`SceneComponent.K2_GetComponentLocation` (`self.Bomb`))))
    (:`then_1`
      (bind _asdestructible_actor (cast `DestructibleActor` OtherActor))
      (`DestructibleComponent.ApplyRadiusDamage` (`DestructibleActor.DestructibleComponent` _asdestructible_actor) 50.0 (`SceneComponent.K2_GetComponentLocation` (`self.Explosion_Radius`)) 300.0 30000.0 false))
    (:`then_2`
      (bind _asblood_dragon_bp (cast `/Game/Fantasy_RPG_Game/Blueprints/Blood_Dragon/Blood_Dragon_BP` OtherActor))
      (`/Game/Fantasy_RPG_Game/Blueprints/Blood_Dragon/Blood_Dragon_BP.Hit_By_Bomb` _asblood_dragon_bp))))

(event `self.ReceiveHit`
  (params (MyComp :type "PrimitiveComponent Object Reference") (Other :type "Actor Object Reference") (OtherComp :type "PrimitiveComponent Object Reference") (bSelfMoved :type Boolean) (HitLocation :type "Vector Structure") (HitNormal :type "Vector Structure") (NormalImpulse :type "Vector Structure") (Hit :type "HitResult Structure (by ref)"))
  (bind _explosion_radius (`self.Explosion_Radius`))
  (bind _radialforce (`self.RadialForce`))
  ;[1 1 1] Destroy_Bomb_BP
  (`|ExecutionSequence`
    (:`then_0`
      (`KismetSystemLibrary.Delay` 1.0)
      ;[1 1 1] Destroy_Bomb_Actor
      (`self.K2_DestroyActor`))
    (:`then_1`
      (`KismetSystemLibrary.Delay` 0.2)
      (`|ExecutionSequence`
        (:`then_0`
          (`/Engine/EditorBlueprintResources/StandardMacros.IsValid` _explosion_radius
            (:`Is Valid`
              (`ActorComponent.K2_DestroyComponent` _explosion_radius))))
        (:`then_1`
          (`/Engine/EditorBlueprintResources/StandardMacros.IsValid` _radialforce
            (:`Is Valid`
              (`ActorComponent.K2_DestroyComponent` _radialforce))))))))

(fn `UserConstructionScript`)